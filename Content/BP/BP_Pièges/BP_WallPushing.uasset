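; BP_WallPushing is a trap Actor whose Cube moves back and forth in an endless loop, acting as a pushing wall.
; On BeginPlay it sets the Timeline's play rate from PlayRate, then a FlipFlop alternates between Play and Reverse, with Finished calling Replay to re-enter it.
; Each Timeline update sets the Cube's relative location to the track value multiplied by the NewLocation X, Y and Z variables.
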(event Custom|replay
  (Utilities|FlowControl|FlipFlop
    (:A
      (bind _newtrack_0 (Timeline|Timeline Play)
        (:Update
          (Transformation|SetRelativeLocation (Variables|Default|GetCube) (Math|Vector|MakeVector (* _newtrack_0 (Variables|Default|GetNew%20Location%20X)) (* _newtrack_0 (Variables|Default|GetNew%20Location%20Y)) (* _newtrack_0 (Variables|Default|GetNew%20Location%20Z))) false false))
        (:Finished
          (CallFunction|Replay))))
    (:B
      (Timeline|Timeline Reverse))))

(event EventBeginPlay
  (Components|Timeline|SetPlayRate (Variables|Default|GetTimeline) (Variables|Default|GetplayRate))
  (Utilities|FlowControl|FlipFlop
    (:A
      (bind _newtrack_0 (Timeline|Timeline Play)
        (:Update
          (Transformation|SetRelativeLocation (Variables|Default|GetCube) (Math|Vector|MakeVector (* _newtrack_0 (Variables|Default|GetNew%20Location%20X)) (* _newtrack_0 (Variables|Default|GetNew%20Location%20Y)) (* _newtrack_0 (Variables|Default|GetNew%20Location%20Z))) false false))
        (:Finished
          (CallFunction|Replay))))
    (:B
      (Timeline|Timeline Reverse))))

(event Collision|EventActorBeginOverlap
  (params (OtherActor :type Actor%20Object%20Reference)))

(event EventTick
  (params (DeltaSeconds :type Float%20%28single-precision%29)))

(fn ConstructionScript)