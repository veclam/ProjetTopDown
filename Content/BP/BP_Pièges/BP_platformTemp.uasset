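; BP_platformTemp is a temporary platform trap that drops after being hit and then resets.
; A hit on the Cube starts a Timeline, used only as a delay, whose Finished output enables physics on the Cube.
; After a fixed wait, physics is disabled and the Cube returns to the location saved at BeginPlay with zeroed rotation.
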(event OnComponentHit(Cube)
  (params (HitComponent :type Primitive%20Component%20Object%20Reference) (OtherActor :type Actor%20Object%20Reference) (OtherComp :type Primitive%20Component%20Object%20Reference) (NormalImpulse :type Vector :default "0, 0, 0") (Hit :type Hit%20Result%20Structure%20%28by%20ref%29))
  (Timeline|Timeline PlayFromStart
    (:Finished
      (Physics|SetSimulatePhysics (Variables|Default|GetCube) true)
      (Utilities|FlowControl|Delay 3.0)
      (Physics|SetSimulatePhysics (Variables|Default|GetCube) false)
      (Transformation|SetWorldLocation (Variables|Default|GetCube) (Variables|Default|GetNewVar) false false)
      (Transformation|SetWorldRotation (Variables|Default|GetCube) "0, 0, 0" false false))))

(event EventBeginPlay
  (Variables|Default|SetNewVar (Transformation|GetWorldLocation (Variables|Default|GetCube))))

(fn ConstructionScript)