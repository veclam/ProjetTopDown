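; Moving platform Blueprint, filed among the traps, that translates and rotates Cube0 along configurable X, Y and Z amounts.
; A launch event sets the timeline play rate, then a FlipFlop alternates between playing and reversing it.
; Two timeline tracks scale the relative location and rotation each update.
; Finishing calls launch again, producing an endless back-and-forth once triggered; nothing in this graph makes the first call.
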(event Custom|launch
  (Components|Timeline|SetPlayRate (Variables|Default|GetTimeline) (Variables|Default|Getplayrate))
  (Utilities|FlowControl|FlipFlop
    (:A
      (bind (_direction _newtrack_0 _newtrack_1) (Timeline|Timeline Play)
        (:Update
          (Transformation|SetRelativeLocation (Variables|Default|Getcube_0) (Math|Vector|MakeVector (* _newtrack_0 (Variables|Default|GetdX)) (* _newtrack_0 (Variables|Default|GetdY)) (* _newtrack_0 (Variables|Default|GetdZ))) false false)
          (Transformation|SetRelativeRotation (Variables|Default|Getcube_0) (Math|Rotator|MakeRotator (* (Variables|Default|GetRotX) _newtrack_1) (* (Variables|Default|GetRotY) _newtrack_1) (* (Variables|Default|GetRotZ) _newtrack_1)) false false))
        (:Finished
          (CallFunction|Launch))))
    (:B
      (Timeline|Timeline Reverse))))

(event Collision|EventActorBeginOverlap
  (params (OtherActor :type Actor%20Object%20Reference)))

(event EventTick
  (params (DeltaSeconds :type Float%20%28single-precision%29)))

(fn ConstructionScript)