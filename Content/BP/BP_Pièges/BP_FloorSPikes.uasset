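; Floor spike trap that repeatedly raises its spikes and kills the player character on contact with its Box trigger.
; After an initial Duration delay on BeginPlay, a timeline drives the relative height of ConeCentrale.
; When the timeline finishes, the cone snaps below its origin, waits briefly, then replays through LaunchSpikes in an endless cycle.
; Any BP_ThirdPersonCharacter that begins overlapping the Box has Death called, with no check on spike state.
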(event OnComponentBeginOverlap(box)
  (params (OverlappedComponent :type Primitive%20Component%20Object%20Reference) (OtherActor :type Actor%20Object%20Reference) (OtherComp :type Primitive%20Component%20Object%20Reference) (OtherBodyIndex :type Integer) (bFromSweep :type Boolean) (SweepResult :type Hit%20Result%20Structure%20%28by%20ref%29))
  (bind _asbp_third_person_character (Utilities|Casting|CastToBP_ThirdPersonCharacter OtherActor))
  (Default|Death _asbp_third_person_character))

(event Custom|launchSpikes
  (bind _activation_des_spikes (Timeline|Timeline PlayFromStart)
    (:Update
      (Transformation|SetRelativeLocation (Variables|Default|GetConeCentrale) (Math|Vector|MakeVector 0.0 0.0 (* _activation_des_spikes 1.4e+02)) false false))
    (:Finished
      (Transformation|SetRelativeLocation (Variables|Default|GetConeCentrale) "0.000000,0.000000,-200.000000" false false)
      (Utilities|FlowControl|Delay 2.0)
      (CallFunction|LaunchSpikes))))

(event EventBeginPlay
  (Utilities|FlowControl|Delay (Variables|Default|GetDuration))
  (bind _activation_des_spikes (Timeline|Timeline Play)
    (:Update
      (Transformation|SetRelativeLocation (Variables|Default|GetConeCentrale) (Math|Vector|MakeVector 0.0 0.0 (* _activation_des_spikes 1.4e+02)) false false))
    (:Finished
      (Transformation|SetRelativeLocation (Variables|Default|GetConeCentrale) "0.000000,0.000000,-200.000000" false false)
      (Utilities|FlowControl|Delay 2.0)
      (CallFunction|LaunchSpikes))))

(event Collision|EventActorBeginOverlap
  (params (OtherActor :type Actor%20Object%20Reference)))

(event EventTick
  (params (DeltaSeconds :type Float%20%28single-precision%29)))

(fn ConstructionScript)