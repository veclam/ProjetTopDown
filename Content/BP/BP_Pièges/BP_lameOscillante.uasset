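; BP_lameOscillante is a swinging blade trap that rotates continuously once play begins.
; A Timeline track scales per-axis roll, pitch and yaw variables to set the root component's relative rotation on each update.
; When the Timeline finishes, a custom event replays it from the start to loop the motion.
; BeginPlay also applies the Playrate variable to the Timeline, controlling the swing speed.
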(event Custom|CustomEvent
  (bind _newtrack_0 (Timeline|Timeline PlayFromStart)
    (:Update
      (Transformation|SetRelativeRotation (Variables|Default|GetDefaultSceneRoot) (Math|Rotator|MakeRotator (* (Variables|Default|GetNew%20Rotation%20X%20%28Roll%29) _newtrack_0) (* (Variables|Default|GetNew%20Rotation%20Y%20%28Pitch%29) _newtrack_0) (* (Variables|Default|GetNew%20Rotation%20Z%20%28Yaw%29) _newtrack_0)) false false))
    (:Finished
      (CallFunction|CustomEvent))))

(event EventBeginPlay
  (Utilities|FlowControl|Sequence
    (:then_0
      (bind _newtrack_0 (Timeline|Timeline Play)
        (:Update
          (Transformation|SetRelativeRotation (Variables|Default|GetDefaultSceneRoot) (Math|Rotator|MakeRotator (* (Variables|Default|GetNew%20Rotation%20X%20%28Roll%29) _newtrack_0) (* (Variables|Default|GetNew%20Rotation%20Y%20%28Pitch%29) _newtrack_0) (* (Variables|Default|GetNew%20Rotation%20Z%20%28Yaw%29) _newtrack_0)) false false))
        (:Finished
          (CallFunction|CustomEvent))))
    (:then_1
      (Utilities|FlowControl|DoOnce false
        (:Completed
          (Components|Timeline|SetPlayRate (Variables|Default|GetTimeline) (Variables|Default|Getplayrate)))))))

(fn ConstructionScript)