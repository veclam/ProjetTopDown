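; BP_fleche is an arrow trap projectile that kills the third-person player character on contact.
; On BeginPlay, a Timeline moves its root from Origin along ForwardVector, scaling a fixed distance by the track value, without sweeping.
; Overlap on either of two capsules casts the other actor to BP_ThirdPersonCharacter and calls Death.
; The arrow destroys itself when the Timeline finishes, not on a hit.
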(event OnComponentBeginOverlap(Capsule)
  (params (OverlappedComponent :type Primitive%20Component%20Object%20Reference) (OtherActor :type Actor%20Object%20Reference) (OtherComp :type Primitive%20Component%20Object%20Reference) (OtherBodyIndex :type Integer) (bFromSweep :type Boolean) (SweepResult :type Hit%20Result%20Structure%20%28by%20ref%29))
  (bind _asbp_third_person_character (Utilities|Casting|CastToBP_ThirdPersonCharacter (stale OnComponentBeginOverlap(Capsule1) OtherActor)))
  (Default|Death _asbp_third_person_character))

(event OnComponentBeginOverlap(Capsule1)
  (params (OverlappedComponent :type Primitive%20Component%20Object%20Reference) (OtherActor :type Actor%20Object%20Reference) (OtherComp :type Primitive%20Component%20Object%20Reference) (OtherBodyIndex :type Integer) (bFromSweep :type Boolean) (SweepResult :type Hit%20Result%20Structure%20%28by%20ref%29))
  (bind _asbp_third_person_character (Utilities|Casting|CastToBP_ThirdPersonCharacter OtherActor))
  (Default|Death _asbp_third_person_character))

(event EventBeginPlay
  (bind _newtrack_0 (Timeline|Timeline Play)
    (:Update
      (Transformation|SetRelativeLocation (Variables|Default|GetDefaultSceneRoot) (+ (Variables|Default|Getorigin) (* _newtrack_0 (* (Variables|Default|Getforward%20vector) 1000))) false false))
    (:Finished
      (Actor|DestroyActor))))

(fn ConstructionScript)